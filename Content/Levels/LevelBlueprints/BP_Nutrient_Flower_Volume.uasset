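; BP_Nutrient_Flower_Volume is a sphere volume that acts as a finite nutrient source for the player's butterfly pawn.
; Overlap opens and closes a Tick-driven gate that, about once a second, moves nutrition into the butterfly at its absorption rate and flashes it green.
; The construction script sizes the sphere, fills the nutrition and binds to the player pawn's death-reset event, which refills it.
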(event `self.ReceiveActorBeginOverlap`
  (params (OtherActor :type "Actor Object Reference"))
  (bind _butterfly_pawn (`self.Butterfly Pawn`))
  (bind _asbppawn_butterfly (cast `/Game/PlayerCharacter/BPPawn_Butterfly` OtherActor))
  (set `self.Butterfly Pawn` _asbppawn_butterfly)
  (if (not (<= (`self.RemainingNutrition`) 0))
    (set `self.isButterflyHere` true)
    (goto _label :!via `Open`)))

(event `self.ReceiveActorEndOverlap`
  (params (OtherActor :type "Actor Object Reference"))
  (bind _butterfly_pawn (`self.Butterfly Pawn`))
  (cast `/Game/PlayerCharacter/BPPawn_Butterfly` OtherActor)
  (set `self.isButterflyHere` false)
  (goto _label :!via `Close`))

(event `self.ReceiveTick`
  (params (DeltaSeconds :type "Float (single-precision)"))
  (bind _butterfly_pawn (`self.Butterfly Pawn`))
  (`/Engine/EditorBlueprintResources/StandardMacros.Gate` true :!label _label
    (:`Exit`
      (if (> (`self.RemainingNutrition`) 0)
        (bind _output_get (set `self.TimeSinceLastEaten` (+ (`self.TimeSinceLastEaten`) DeltaSeconds)))
        (if (>= _output_get 1.0)
          (set `self.RemainingNutrition` (- (`self.RemainingNutrition`) (`/Game/PlayerCharacter/BPPawn_Butterfly.NutrientAbsorbsion` _butterfly_pawn)))
          (set `/Game/PlayerCharacter/BPPawn_Butterfly.StoredNutrients` (+ (`/Game/PlayerCharacter/BPPawn_Butterfly.StoredNutrients` _butterfly_pawn) (`/Game/PlayerCharacter/BPPawn_Butterfly.NutrientAbsorbsion` _butterfly_pawn)) _butterfly_pawn)
          (set `self.TimeSinceLastEaten` 0.0)
          (`/Game/PlayerCharacter/BPPawn_Butterfly.FlashGreen` _butterfly_pawn))))))

(event `Bind Reset`
  (add `/Game/PlayerCharacter/BPPawn_Butterfly.ResetOnDeath` (cast `/Game/PlayerCharacter/BPPawn_Butterfly` (`Controller.K2_GetPawn` (`GameplayStatics.GetPlayerController` 0)) :!pure true) (delegate `ResetOnDeath_Event`)))

(event `ResetOnDeath_Event`
  (set `self.RemainingNutrition` (`self.StoredNutrition`)))

(fn `UserConstructionScript`
  (`SphereComponent.SetSphereRadius` (`self.Sphere`) (`self.Radius`) true)
  (set `self.RemainingNutrition` (`self.StoredNutrition`))
  (`self.Bind Reset`))