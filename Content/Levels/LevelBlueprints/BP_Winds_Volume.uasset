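; BP_Winds_Volume is a wind zone that pushes the player's butterfly pawn downward while it is inside.
; Collision box overlaps with BPPawn_Butterfly store the pawn and toggle an IsBlowing flag.
; While the flag is set, Tick adds a fixed downward LaunchCharacter velocity every frame, without delta-time scaling.
; The construction script sizes the box from LengthOfWind and HeightOfWind with a fixed depth.
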(event `self.Collision.OnComponentBeginOverlap`
  (params (OverlappedComponent :type "PrimitiveComponent Object Reference") (OtherActor :type "Actor Object Reference") (OtherComp :type "PrimitiveComponent Object Reference") (OtherBodyIndex :type Integer) (bFromSweep :type Boolean) (SweepResult :type "HitResult Structure (by ref)"))
  (bind _asbppawn_butterfly (cast `/Game/PlayerCharacter/BPPawn_Butterfly` OtherActor))
  (set `self.isBlowing` true))

(event `self.Collision.OnComponentEndOverlap`
  (params (OverlappedComponent :type "PrimitiveComponent Object Reference") (OtherActor :type "Actor Object Reference") (OtherComp :type "PrimitiveComponent Object Reference") (OtherBodyIndex :type Integer))
  (cast `/Game/PlayerCharacter/BPPawn_Butterfly` OtherActor)
  (set `self.isBlowing` false))

(event `self.ReceiveTick`
  (params (DeltaSeconds :type "Float (single-precision)"))
  (if (`self.isBlowing`)
    (`Character.LaunchCharacter` (stale `self.Collision.OnComponentBeginOverlap` _asbppawn_butterfly) (0.0 0.0 -100.0) false false)))

(fn `UserConstructionScript`
  (`BoxComponent.SetBoxExtent` (`self.Collision`) (`KismetMathLibrary.MakeVector` (`self.Length Of Wind`) 32.0 (`self.Height of Wind`)) true))