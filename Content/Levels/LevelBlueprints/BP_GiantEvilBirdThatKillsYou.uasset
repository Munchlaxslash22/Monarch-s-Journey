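; BP_GiantEvilBirdThatKillsYou is a hazard actor that drops its cube when a butterfly pawn is detected beneath it.
; Each tick it traces downward by DropDistance with the Pawn profile, drawing and printing debug output.
; A butterfly hit restarts the Dropdown timeline, which places the cube at the hit's X and Y, with hit Z scaled by the timeline value.
; No kill or damage logic appears.
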(event `self.ReceiveTick`
  (params (DeltaSeconds :type "Float (single-precision)"))
  (bind _returnvalue (`self.K2_GetActorLocation`))
  (bind (_outhit _returnvalue_2) (`KismetSystemLibrary.LineTraceSingleByProfile` :`Start` _returnvalue :`End` (`KismetMathLibrary.MakeVector` (.x _returnvalue) (.y _returnvalue) (- (.z _returnvalue) (`self.DropDistance`))) :`ProfileName` "Pawn" :`DrawDebugType` "ForDuration"))
  (`KismetSystemLibrary.PrintString` "Hello" _returnvalue_2)
  (cast `/Game/PlayerCharacter/BPPawn_Butterfly` (`.HitActor` (`GameplayStatics.BreakHitResult` _outhit)))
  (`self.Drop`))

(event `Drop`
  (bind (_direction _distancedropped) (`Timeline|Dropdown` :`NewTime` 3.0 :!via `PlayFromStart`)
    (:`Update`
      (`SceneComponent.K2_SetWorldLocation` (`self.Cube`) (`KismetMathLibrary.MakeVector` (.x (`.Location` (`GameplayStatics.BreakHitResult` (stale `self.ReceiveTick` _outhit)))) (.y (`.Location` (`GameplayStatics.BreakHitResult` (stale `self.ReceiveTick` _outhit)))) (* (.z (`.Location` (`GameplayStatics.BreakHitResult` (stale `self.ReceiveTick` _outhit)))) _distancedropped)) false false))))

(fn `UserConstructionScript`)